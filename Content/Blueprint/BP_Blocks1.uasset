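; BP_Blocks1 is a moving block actor that scrolls along negative X, likely an obstacle in a side-scrolling game.
; On BeginPlay it shifts its root by a random vertical offset so each instance appears at a different height.
; Each Tick moves the root at a constant, frame-rate-independent speed by setting world location without sweep, so it does not stop on collisions.
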(event EventBeginPlay
  (Transformation|SetWorldLocation (Variables|Default|GetDefaultSceneRoot) (+ (Transformation|GetWorldLocation (Variables|Default|GetDefaultSceneRoot)) (Math|Vector|MakeVector 0.0 0.0 (Math|Random|RandomFloatinRange -3.5e+02 3.5e+02))) false false))

(event EventTick
  (params (DeltaSeconds :type Float%20%28single-precision%29))
  (Transformation|SetWorldLocation (Variables|Default|GetDefaultSceneRoot) (+ (Transformation|GetWorldLocation (Variables|Default|GetDefaultSceneRoot)) (Math|Vector|MakeVector (* DeltaSeconds (Math|Float|MakeLiteralFloat -6e+02)) 0.0 0.0)) false false))

(fn ConstructionScript)