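; Player bird for a Flappy Bird-style Paper2D game, driven by capsule physics.
; Tick adds a delta-scaled downward force, while Jump calls NewJump, which zeroes velocity (its added force is zero), and briefly swaps the sprite.
; The first overlap kills the bird, spins it with torque and, after a delay, lets Jump reload Level1.
; Jump and restart require IsPlaying, which this graph never sets true.
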(event Collision|EventActorBeginOverlap
  (params (OtherActor :type Actor%20Object%20Reference))
  (if (Variables|Default|GetisAlive)
    (Variables|Default|SetisAlive false)
    (CallFunction|NewJump)
    (Class|PrimitiveComponent|AddTorqueinDegrees (Variables|Default|GetCapsule) "0.000000,-10000000.000000,0.000000" "None" false)
    (Utilities|FlowControl|Delay 1.0)
    (Variables|Default|SetReadytoRestart true)))

(event EventBeginPlay
  (Physics|SetEnableGravity (Variables|Default|GetCapsule) true))

(event EventTick
  (params (DeltaSeconds :type Float%20%28single-precision%29))
  (Physics|AddForce (Variables|Default|GetCapsule) (Math|Vector|MakeVector 0.0 0.0 (* (Math|Float|MakeLiteralFloat -1.2e+05) DeltaSeconds)) "None" false))

(event Input|ActionEvents|InputActionJump
  (params (Key :type Key%20Structure :default "None"))
  (:Pressed
    (Utilities|FlowControl|Sequence
      (:then_0
        (if (Variables|Default|GetisPlaying)
          (if (Variables|Default|GetisAlive)
            (CallFunction|NewJump)
            (elif (Variables|Default|GetReadytoRestart)
              (Game|OpenLevel(byName) "Level1")))
          (else
            (Variables|Default|SetisPlaying false)
            (Physics|SetEnableGravity (Variables|Default|GetCapsule) true))))
      (:then_1
        (if (Variables|Default|GetisAlive)
          (Rendering|Components|Sprite|SetSprite (Variables|Default|GetPaperSprite) "/Game/Level1/bird/Bird1-1_Sprite_3.Bird1-1_Sprite_3")
          (Utilities|FlowControl|Delay 0.2)
          (Rendering|Components|Sprite|SetSprite (Variables|Default|GetPaperSprite) "/Game/Level1/bird/Bird1-1_Sprite_0.Bird1-1_Sprite_0"))))))

(fn ConstructionScript)

(fn NewJump
  (Physics|SetPhysicsLinearVelocity (Variables|Default|GetCapsule) "0, 0, 0" false "None")
  (Physics|AddForce (Variables|Default|GetCapsule) "0, 0, 0" "None" false))