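; GreenPipe_BP is a scrolling pipe obstacle with a Plum score pickup, in the style of Flappy Bird.
; On BeginPlay it shifts its root by a random vertical offset, then moves it along negative X each Tick at a constant speed scaled by delta time.
; Any overlap with Plum calls AddPoint on GameMode_BP and destroys that component, so each pipe scores only once.
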(event OnComponentBeginOverlap(Plum)
  (params (OverlappedComponent :type Primitive%20Component%20Object%20Reference) (OtherActor :type Actor%20Object%20Reference) (OtherComp :type Primitive%20Component%20Object%20Reference) (OtherBodyIndex :type Integer) (bFromSweep :type Boolean) (SweepResult :type Hit%20Result%20Structure%20%28by%20ref%29))
  (bind _asgame_mode_bp (Utilities|Casting|CastToGameMode_BP (Game|GetGameMode)))
  (Default|AddPoint _asgame_mode_bp)
  (Components|DestroyComponent (Variables|Default|GetPlum)))

(event EventTick
  (params (DeltaSeconds :type Float%20%28single-precision%29))
  (Transformation|SetWorldLocation (Variables|Default|GetDefaultSceneRoot) (+ (Transformation|GetWorldLocation (Variables|Default|GetDefaultSceneRoot)) (Math|Vector|MakeVector (* DeltaSeconds (Math|Float|MakeLiteralFloat -5e+02)) 0.0 0.0)) false false))

(event EventBeginPlay
  (Transformation|SetWorldLocation (Variables|Default|GetDefaultSceneRoot) (+ (Transformation|GetWorldLocation (Variables|Default|GetDefaultSceneRoot)) (Math|Vector|MakeVector 0.0 0.0 (Math|Random|RandomFloatinRange -2.8e+02 2.8e+02))) false false))

(fn ConstructionScript)