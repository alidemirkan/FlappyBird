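; Player bird for a Flappy Bird-style game, driven by physics on its capsule.
; The first Jump press enables gravity; later presses reset velocity and apply an upward force, with a brief sprite swap for the flap.
; Tick adds extra downward force while falling.
; Overlapping a component tagged Pipe kills the bird with a hop and spin, after which Jump reloads FlappyMap.
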(event OnComponentBeginOverlap(CapsuleCollision)
  (params (OverlappedComponent :type Primitive%20Component%20Object%20Reference) (OtherActor :type Actor%20Object%20Reference) (OtherComp :type Primitive%20Component%20Object%20Reference) (OtherBodyIndex :type Integer) (bFromSweep :type Boolean) (SweepResult :type Hit%20Result%20Structure%20%28by%20ref%29))
  (Utilities|IsValid OtherComp
    (:Is%20Valid
      (if (Components|ComponentHasTag OtherComp "Pipe")
        (if (Variables|Default|GetisAlive)
          (Variables|Default|SetisAlive false)
          (Physics|SetPhysicsLinearVelocity (Variables|Default|GetCapsuleCollision) "0, 0, 0" false "None")
          (Physics|AddForce (Variables|Default|GetCapsuleCollision) "0.000000,0.000000,29500.000000" "None" false)
          (Class|PrimitiveComponent|AddTorqueinDegrees (Variables|Default|GetCapsuleCollision) "0.000000,-20000000.000000,0.000000" "None" false))))))

(event EventTick
  (params (DeltaSeconds :type Float%20%28single-precision%29))
  (bind _returnvalue (Physics|GetPhysicsLinearVelocity (Variables|Default|GetCapsuleCollision) "None"))
  (if (> 0.0 (.z _returnvalue))
    (Physics|AddForce (Variables|Default|GetCapsuleCollision) (Math|Vector|MakeVector 0.0 0.0 (* (Math|Float|MakeLiteralFloat -3e+04) DeltaSeconds)) "None" false)))

(event EventBeginPlay
  (Physics|SetEnableGravity (Variables|Default|GetCapsuleCollision) false)
  (Audio|PlaySound2D "/Game/Sounds/NewSoundCue.NewSoundCue" 1.0 1.0 0.0 0 0))

(event Input|ActionEvents|InputActionJump
  (params (Key :type Key%20Structure :default "None"))
  (:Pressed
    (Utilities|FlowControl|Sequence
      (:then_0
        (if (Variables|Default|GetisPlaying)
          (if (Variables|Default|GetisAlive)
            (Physics|SetPhysicsLinearVelocity (Variables|Default|GetCapsuleCollision) "0, 0, 0" false "None")
            (Physics|AddForce (Variables|Default|GetCapsuleCollision) "0.000000,0.000000,29500.000000" "None" false)
            (else
              (Game|OpenLevel(byName) "FlappyMap")))
          (else
            (Variables|Default|SetisPlaying true)
            (Physics|SetEnableGravity (Variables|Default|GetCapsuleCollision) true))))
      (:then_1
        (if (Variables|Default|GetisAlive)
          (Rendering|Components|Sprite|SetSprite (Variables|Default|GetPaperSprite) "/Game/Assets/Player/StyleBird2/Bird2-6_Sprite_0.Bird2-6_Sprite_0")
          (Utilities|FlowControl|Delay 0.2)
          (Rendering|Components|Sprite|SetSprite (Variables|Default|GetPaperSprite) "/Game/Assets/Player/StyleBird2/Bird2-6_Sprite_1.Bird2-6_Sprite_1"))))))

(fn ConstructionScript)